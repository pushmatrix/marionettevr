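; VR hand Blueprint for MarionetteVR that pinches string nubs or grips handles, holding one item at a time.
; Pinch and grip starts pick the closest overlapping component tagged pinchable (pinch hitbox) or grabbable (hand mesh), storing its owner as HeldItem.
; Grab and release behavior is delegated to that object through BPI_Grabbable.
; A gate per input lets an end event release only after its matching start.
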(event `OnPinchEnd`
  (bind _returnvalue (`KismetSystemLibrary.Conv_InterfaceToObject` (`self.HeldItem`)))
  (`|ExecutionSequence`
    (:`then_0`
      ;[1 1 1] This makes it so the pinch end will only be able to run if a pinch start has preceded it.
      (`/Engine/EditorBlueprintResources/StandardMacros.Gate` true :!label _label
        (:`Exit`
          (`/Engine/EditorBlueprintResources/StandardMacros.IsValid` _returnvalue :!label _label_2
            (:`Is Valid`
              ;[1 1 1] Defer logic for what happens on release to the object being released.
              (message `/Game/MarionetteVR/Core/BPI_Grabbable.OnRelease` _returnvalue self)
              (set `self.HeldItem` null))))))
    (:`then_1`
      (goto _label :!via `Close`))))

(event `OnPinchStart`
  (bind _pinchhitbox (`self.PinchHitbox`))
  ;[1 1 1] Can't pinch something if you are already holding something.
  (`/Engine/EditorBlueprintResources/StandardMacros.IsValid` (`KismetSystemLibrary.Conv_InterfaceToObject` (`self.HeldItem`))
    (:`Is Not Valid`
      ;[1 1 1] Only the little "nubs" that the strings are attached to  have the tag = pinchable
      (bind _closestgrabbable (`self.GetClosestGrabbableByTag` (`PrimitiveComponent.GetOverlappingComponents` _pinchhitbox) (`SceneComponent.K2_GetComponentLocation` _pinchhitbox) "pinchable"))
      (set `self.HeldItem` _closestgrabbable)
      (`|ExecutionSequence`
        (:`then_0`
          (goto _label :!via `Open`))
        (:`then_1`
          (`/Engine/EditorBlueprintResources/StandardMacros.IsValid` (`KismetSystemLibrary.Conv_InterfaceToObject` (`self.HeldItem`)) :!label _label_3
            (:`Is Valid`
              ;[1 1 1] Defer the logic for what happens when an object is grabbed/pinched to the object itself. They will implement the Grabbable interface.
              (message `/Game/MarionetteVR/Core/BPI_Grabbable.OnGrab` (`KismetSystemLibrary.Conv_InterfaceToObject` (`self.HeldItem`)) self))))))))

(event `OnGripStart`
  (bind _skeletalmesh (`self.SkeletalMesh`))
  ;[1 1 1] Can't grab something if you are already holding/pinching something.
  (`/Engine/EditorBlueprintResources/StandardMacros.IsValid` (`KismetSystemLibrary.Conv_InterfaceToObject` (`self.HeldItem`))
    (:`Is Not Valid`
      ;[1 1 1] Only the handle should have tag = grabbable
      (bind _closestgrabbable (`self.GetClosestGrabbableByTag` (`PrimitiveComponent.GetOverlappingComponents` _skeletalmesh) (`SceneComponent.K2_GetComponentLocation` _skeletalmesh) "grabbable"))
      (set `self.HeldItem` _closestgrabbable)
      (`|ExecutionSequence`
        (:`then_0`
          (goto _label_4 :!via `Open`))
        (:`then_1`
          (goto _label_3))))))

(event `OnGripEnd`
  (`|ExecutionSequence`
    (:`then_0`
      ;[1 1 1] This makes it so the grip end will only be able to run if a grip start has preceded it.
      (`/Engine/EditorBlueprintResources/StandardMacros.Gate` true :!label _label_4
        (:`Exit`
          (goto _label_2))))
    (:`then_1`
      (goto _label_4 :!via `Close`))))

(fn `GetClosestGrabbableByTag`
  (params (Components :type "Array of ActorComponent Object Reference") (Location :type "Vector Structure") (Tag :type Name))
  (returns (ClosestGrabbable :type "/Game/MarionetteVR/Core/BPI_Grabbable Interface"))
  (locals (ClosestDistance :type "Float (double-precision)" :default 9999999.0) (ClosestComponent :type "ActorComponent Object Reference") (TargetLocation :type "Vector Structure") (CurrentComponent :type "PrimitiveComponent Object Reference"))
  (bind _closestcomponent (`local.ClosestComponent`))
  (set `local.TargetLocation` Location)
  (for _array_element Components
    (if (`ActorComponent.ComponentHasTag` _array_element Tag)
      (bind _asprimitive_component (cast `PrimitiveComponent` _array_element))
      (bind _output_get (set `local.CurrentComponent` _asprimitive_component))
      (bind _returnvalue (`KismetMathLibrary.VSize` (- (`local.TargetLocation`) (`SceneComponent.K2_GetComponentLocation` _output_get))))
      (if (< _returnvalue (`local.ClosestDistance`))
        (set `local.ClosestDistance` _returnvalue)
        (set `local.ClosestComponent` (`local.CurrentComponent`)))))
  (`/Engine/EditorBlueprintResources/StandardMacros.IsValid` _closestcomponent
    (:`Is Valid`
      (bind _asbpi_grabbable (cast `/Game/MarionetteVR/Core/BPI_Grabbable` (`ActorComponent.GetOwner` _closestcomponent))
        (:`then`
          (return _asbpi_grabbable))
        (:`CastFailed`
          (return null))))
    (:`Is Not Valid`
      (return null))))

(fn `UserConstructionScript`)