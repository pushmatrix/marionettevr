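; BP_Nub is a grabbable nub for the VR marionette that can be pulled from its holder and put back.
; It moves its parent component, whose relative transform and attach parent are cached on BeginPlay.
; Grabbing snaps that component to the hand's pinch hitbox.
; On release it reattaches and resets if near its original spot on the holder, otherwise it detaches and hangs in midair.
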(event `self.ReceiveBeginPlay`
  (bind _returnvalue (`self.GetParentComponent`))
  ;[1 1 1] Store its beginning transform so that we know how to reset it when someone brings the nub back
  (set `self.StartingTransform` (`SceneComponent.GetRelativeTransform` _returnvalue))
  (set `self.StartingAttachment` (`SceneComponent.GetAttachParent` _returnvalue)))

(event `/Game/MarionetteVR/Core/BPI_Grabbable.OnGrab`
  (params (OwningHand :type "/Game/MarionetteVR/Core/Hands/BP_Hand Object Reference"))
  ;[1 1 1] Grab
  (`SceneComponent.K2_AttachToComponent` (`KismetArrayLibrary.Array_Get` (`SceneComponent.GetParentComponents` (`self.Nub`))) (`/Game/MarionetteVR/Core/Hands/BP_Hand.PinchHitbox` OwningHand) "None" "SnapToTarget" "SnapToTarget" "KeepWorld" true))

(event `/Game/MarionetteVR/Core/BPI_Grabbable.OnRelease`
  (params (OwningHand :type "/Game/MarionetteVR/Core/Hands/BP_Hand Object Reference"))
  ;[1 1 1] If the nub is close enough to its starting placement when it is released, return it to its beginning location
  (if (< (`KismetMathLibrary.VSize` (- (`SceneComponent.K2_GetComponentLocation` (`self.GetParentComponent`)) (`KismetMathLibrary.TransformLocation` (`SceneComponent.K2_GetComponentToWorld` (`self.StartingAttachment`)) (.location (`self.StartingTransform`))))) 10.0)
    (`SceneComponent.K2_AttachToComponent` (`self.GetParentComponent`) (`self.StartingAttachment`) "None" "KeepWorld" "KeepWorld" "KeepWorld" true)
    (`SceneComponent.K2_SetRelativeTransform` (`self.GetParentComponent`) (`self.StartingTransform`) false false)
    (else
      ;[1 1 1] If the nub is too far from its original spot, let it hang in midair
      (`SceneComponent.K2_DetachFromComponent` (`self.GetParentComponent`) "KeepWorld" "KeepWorld" "KeepWorld" true))))

(fn `UserConstructionScript`)